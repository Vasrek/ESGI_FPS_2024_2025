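; BP_Enemy is a spider enemy that patrols random reachable points, chases the player and attacks in melee.
; AI perception switches it between a faster chase that ends in an attack montage and a slower patrol.
; A sphere overlap damages the player then disables its own collision, which starts off and is not re-enabled in this graph.
; Incoming damage reduces health with a hit montage, or destroys the actor at zero.
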(event OnTargetPerceptionUpdated(AIPerception)
  (params (Actor :type Actor%20Object%20Reference) (Stimulus :type AI%20Stimulus%20Structure))
  (bind _asbp_player (Utilities|Casting|CastToBP_Player Actor))
  (if (.bsuccessfullysensed Stimulus)
    (Variables|/Script/Engine.CharacterMovementComponent|SetMaxWalkSpeed (Variables|Character|GetCharacterMovement) 4e+02)
    (AI|AIMoveTo self "0, 0, 0" _asbp_player 1.5e+02 true
      (:OnSuccess
        (Animation|PlayAnimMontage "/Game/StylizedCreaturesBundle/Animations/Spider/AM_Spider_Attack.AM_Spider_Attack" 1.0 "None")
        (Utilities|FlowControl|Delay 1.5)))
    (else
      (CallFunction|Patrol)
      (Variables|/Script/Engine.CharacterMovementComponent|SetMaxWalkSpeed (Variables|Character|GetCharacterMovement) 2e+02))))

(event OnComponentBeginOverlap(Sphere)
  (params (OverlappedComponent :type Primitive%20Component%20Object%20Reference) (OtherActor :type Actor%20Object%20Reference) (OtherComp :type Primitive%20Component%20Object%20Reference) (OtherBodyIndex :type Integer) (bFromSweep :type Boolean) (SweepResult :type Hit%20Result%20Structure%20%28by%20ref%29))
  (bind _asbp_player (Utilities|Casting|CastToBP_Player OtherActor))
  (Default|PlayerDamage _asbp_player (Variables|Default|GetAttackDamage))
  (Collision|SetCollisionEnabled (Variables|Default|GetSphere) "NoCollision"))

(event Custom|Damage
  (params (DamageToApply :type Float%20%28double-precision%29))
  (if (<= (- (Variables|Default|GetHealth) DamageToApply) 0.0)
    (CallFunction|Death)
    (else
      (Variables|Default|SetHealth (- (Variables|Default|GetHealth) DamageToApply))
      (Animation|PlayAnimMontage "/Game/StylizedCreaturesBundle/Animations/Spider/AM_Spider_Hit.AM_Spider_Hit" 1.0 "None"))))

(event Custom|Death
  (Actor|DestroyActor))

(event Custom|Patrol
  (AI|AIMoveTo self (.RandomLocation (AI|Navigation|GetRandomReachablePointinRadius (Transformation|GetActorLocation) 1e+03 0 0)) 0 5.0 false :!label _label
    (:OnSuccess
      (Utilities|FlowControl|Delay 3.0)
      (goto _label))))

(event EventBeginPlay
  (CallFunction|Patrol)
  (Collision|SetCollisionEnabled (Variables|Default|GetSphere) "NoCollision"))

(fn ConstructionScript)