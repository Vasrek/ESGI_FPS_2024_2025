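; First-person player Blueprint handling movement, weapon pickup, shooting, reloading, health and a HUD overlay.
; Enhanced Input drives actions; equipping attaches the overlapped weapon to a hand socket and hides the pickup prompt.
; Firing spawns bullets at the muzzle socket, re-calling itself after a fire-rate delay for automatics, and reloads from reserve ammo when empty.
; Damage updates the overlay and restarts the level at zero health, with U as a test damage key.
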(event Custom|AddPickupWidgetOnScreen
  (params (OverlapWeapon :type BP%20Weapon%20Object%20Reference))
  ;[1 1 1] Handle pickup widget
  (Utilities|IsValid (Variables|Default|GetPickupWidgetRef)
    (:Is%20Valid
      _)
    (:Is%20Not%20Valid
      (bind _returnvalue (UserInterface|CreateWidget "/Game/01-Blueprints/Widgets/WBP_Pickup.WBP_Pickup_C"))
      (bind _output_get (Variables|Default|SetPickupWidgetRef _returnvalue))
      (UserInterface|Viewport|AddtoViewport _output_get 0)))
  (Variables|/Script/UMG.Widget|SetVisibility (Variables|Default|GetPickupWidgetRef) "Visible")
  (Variables|Default|SetOverlapWeapon OverlapWeapon))

(event Custom|HidePickUpWidget
  (bind _pickupwidgetref (Variables|Default|GetPickupWidgetRef))
  ;[1 1 1] Handle pickup widget
  (Utilities|IsValid _pickupwidgetref
    (:Is%20Valid
      (Variables|/Script/UMG.Widget|SetVisibility _pickupwidgetref "Hidden")
      (Variables|Default|SetOverlapWeapon 0))))

(event Custom|FireWeapon
  (bind _equippedweapon (Variables|Default|GetEquippedWeapon))
  (bind _playeroverlayref (Variables|Default|GetPlayerOverlayRef))
  (bind _equippedweapon_2 (Variables|Default|GetEquippedWeapon))
  (bind _weaponmesh (Variables|/Game/01-Blueprints/Weapons/BP_Weapon.BP_Weapon_C|GetWeaponMesh _equippedweapon))
  ;[1 1 1] Fire input action - play animation - spawn bullet
  (if (Variables|Default|GetCanFire?)
    (Utilities|CheckCurrentAmmo?
      (:HaveAmmo
        (Variables|Default|SetCanFire? false)
        (Utilities|IsValid _equippedweapon
          (:Is%20Valid
            (Variables|Default|SetisFiring? true)
            (Components|Animation|PlayAnimation (Variables|Default|GetFirstPersonMesh) "/Game/FirstPersonArms/Animations/FP_Rifle_Fire.FP_Rifle_Fire" false)
            (Utilities|IsValid _weaponmesh
              (:Is%20Valid
                (Components|Animation|PlayAnimation _weaponmesh "/Game/MilitaryWeapSilver/Weapons/Animations/Fire_Rifle_W.Fire_Rifle_W" false)
                (Game|SpawnActorfromClass "/Game/01-Blueprints/Weapons/Bullets/BP_Bullets.BP_Bullets_C" (Math|Transform|MakeTransform (Transformation|GetSocketLocation (Variables|/Game/01-Blueprints/Weapons/BP_Weapon.BP_Weapon_C|GetWeaponMesh (Variables|Default|GetEquippedWeapon)) "BulletSpawn") (Transformation|GetSocketRotation (Variables|/Game/01-Blueprints/Weapons/BP_Weapon.BP_Weapon_C|GetWeaponMesh (Variables|Default|GetEquippedWeapon)) "BulletSpawn") "1.000000,1.000000,1.000000") "AdjustIfPossibleButAlwaysSpawn" "MultiplyWithRoot" 0 0)
                (bind _result (Math|Integer|DecrementInt (Variables|/Game/01-Blueprints/Weapons/BP_Weapon.BP_Weapon_C|GetAmmo _equippedweapon_2))
                  (:%20%20
                    (Utilities|IsValid _playeroverlayref
                      (:Is%20Valid
                        (Default|UpdateAmmoText _playeroverlayref _result (Variables|Default|GetARAmmo))
                        (Utilities|FlowControl|Delay (Variables|/Game/01-Blueprints/Weapons/BP_Weapon.BP_Weapon_C|GetFireRate _equippedweapon_2))
                        (Variables|Default|SetCanFire? true)
                        (if (and (Variables|/Game/01-Blueprints/Weapons/BP_Weapon.BP_Weapon_C|GetisAutomatic? _equippedweapon_2) (Variables|Default|GetisFiring?))
                          (CallFunction|FireWeapon)))))))))))
      (:NoAmmoLeft
        (CallFunction|Reload)
        (Variables|Default|SetisFiring? false)))))

(event Custom|Reload
  (bind _equippedweapon (Variables|Default|GetEquippedWeapon))
  (bind _playeroverlayref (Variables|Default|GetPlayerOverlayRef))
  (bind _equippedweapon_2 (Variables|Default|GetEquippedWeapon))
  ;[1 1 1] Reload
  (if (not (Variables|Default|GetisReloading?))
    (Variables|Default|SetisReloading? true)
    (Variables|Default|SetCanFire? false)
    (Utilities|IsValid _equippedweapon_2
      (:Is%20Valid
        (bind _output_get (Variables|Default|SetARAmmo (+ (Variables|Default|GetARAmmo) (Variables|/Game/01-Blueprints/Weapons/BP_Weapon.BP_Weapon_C|GetAmmo _equippedweapon_2))))
        (if (> _output_get 0)
          (if (< (- (Variables|Default|GetARAmmo) (Variables|/Game/01-Blueprints/Weapons/BP_Weapon.BP_Weapon_C|GetMaxAmmo _equippedweapon_2)) 0)
            (Variables|Default|SetARAmmo (* (Variables|Default|GetARAmmo) -1)))
          (bind _output_get_2 (Variables|/Game/01-Blueprints/Weapons/BP_Weapon.BP_Weapon_C|SetAmmo (Variables|Default|GetEquippedWeapon) (Math|Integer|Clamp(Integer) (Variables|Default|GetARAmmo) 0 (Variables|/Game/01-Blueprints/Weapons/BP_Weapon.BP_Weapon_C|GetMaxAmmo (Variables|Default|GetEquippedWeapon)))))
          (if (> (- _output_get_2 (Variables|Default|GetARAmmo)) 0)
            (Variables|/Game/01-Blueprints/Weapons/BP_Weapon.BP_Weapon_C|SetAmmo (Variables|Default|GetEquippedWeapon) (- _output_get_2 (Variables|Default|GetARAmmo)))
            (Variables|Default|SetARAmmo 0)
            (else
              (Variables|Default|SetARAmmo (* (- _output_get_2 (Variables|Default|GetARAmmo)) -1))))
          (Utilities|IsValid _playeroverlayref
            (:Is%20Valid
              (Default|UpdateAmmoText _playeroverlayref (Variables|/Game/01-Blueprints/Weapons/BP_Weapon.BP_Weapon_C|GetAmmo _equippedweapon) (Variables|Default|GetARAmmo))
              (Utilities|FlowControl|Delay (Variables|/Game/01-Blueprints/Weapons/BP_Weapon.BP_Weapon_C|GetReloadCD _equippedweapon))
              (Variables|Default|SetCanFire? true)
              (Variables|Default|SetisReloading? false))))))))

(event Custom|PlayerDamage
  (params (DamageToApply :type Float%20%28double-precision%29))
  (bind _playeroverlayref (Variables|Default|GetPlayerOverlayRef))
  (bind _output_get (Variables|Default|SetCurrentHealth (- (Variables|Default|GetCurrentHealth) DamageToApply)))
  (if (<= _output_get 0.0)
    (Variables|Default|SetCurrentHealth 0.0)
    (CallFunction|Death))
  (Utilities|IsValid _playeroverlayref
    (:Is%20Valid
      (Default|UpdateHealth _playeroverlayref (Variables|Default|GetCurrentHealth) (Variables|Default|GetMaxHealth)))))

(event Custom|Death
  (Development|ExecuteConsoleCommand "RestartLevel" 0))

(event Input|EnhancedActionEvents|EnhancedInputActionIA_Player_Move
  (params (ActionValue :type Vector%202D%20Structure) (ElapsedSeconds :type Float%20%28double-precision%29) (TriggeredSeconds :type Float%20%28double-precision%29) (InputAction :type Input%20Action%20Object%20Reference :default "/Game/01-Blueprints/Inputs/Actions/IA_Player_Move.IA_Player_Move"))
  ;[1 1 1] Player move input
  (Pawn|Input|AddMovementInput (Transformation|GetActorRightVector) (.x ActionValue) false)
  (Pawn|Input|AddMovementInput (Transformation|GetActorForwardVector) (.y ActionValue) false))

(event Input|EnhancedActionEvents|EnhancedInputActionIA_Player_Look
  (params (ActionValue :type Vector%202D%20Structure) (ElapsedSeconds :type Float%20%28double-precision%29) (TriggeredSeconds :type Float%20%28double-precision%29) (InputAction :type Input%20Action%20Object%20Reference :default "/Game/01-Blueprints/Inputs/Actions/IA_Player_Look.IA_Player_Look"))
  ;[1 1 1] Player look input (camera)
  (Pawn|Input|AddControllerYawInput (.x ActionValue))
  (Pawn|Input|AddControllerPitchInput (.y ActionValue)))

(event Input|EnhancedActionEvents|EnhancedInputActionIA_Player_Jump
  (params (ActionValue :type Boolean) (ElapsedSeconds :type Float%20%28double-precision%29) (TriggeredSeconds :type Float%20%28double-precision%29) (InputAction :type Input%20Action%20Object%20Reference :default "/Game/01-Blueprints/Inputs/Actions/IA_Player_Jump.IA_Player_Jump"))
  ;[1 1 1] Player jump input
  (:Started
    (Character|Jump))
  (:Completed
    (Character|StopJumping)))

(event Input|EnhancedActionEvents|EnhancedInputActionIA_Player_Equip
  (params (ActionValue :type Boolean) (ElapsedSeconds :type Float%20%28double-precision%29) (TriggeredSeconds :type Float%20%28double-precision%29) (InputAction :type Input%20Action%20Object%20Reference :default "/Game/01-Blueprints/Inputs/Actions/IA_Player_Equip.IA_Player_Equip"))
  (bind _overlapweapon (Variables|Default|GetOverlapWeapon))
  (bind _playeroverlayref (Variables|Default|GetPlayerOverlayRef))
  (bind _overlapweapon_2 (Variables|Default|GetOverlapWeapon))
  ;[1 1 1] Equip overlaping weapon and attach it to right hand socket - hide pickup widget
  (:Started
    (Utilities|IsValid _overlapweapon
      (:Is%20Valid
        (Transformation|AttachComponentToComponent _overlapweapon (Variables|Default|GetFirstPersonMesh) "HandR_Socket" "SnapToTarget" "KeepRelative" "KeepRelative" true)
        (Variables|/Game/01-Blueprints/Weapons/BP_Weapon.BP_Weapon_C|SetisEquipped? _overlapweapon_2 true)
        (Variables|Default|SetEquippedWeapon _overlapweapon_2)
        (CallFunction|HidePickUpWidget)
        (Variables|Default|SetCanFire? true)
        (Utilities|IsValid (Variables|Default|GetEquippedWeapon)
          (:Is%20Valid
            (Utilities|IsValid _playeroverlayref
              (:Is%20Valid
                (Default|UpdateAmmoText _playeroverlayref (Variables|/Game/01-Blueprints/Weapons/BP_Weapon.BP_Weapon_C|GetAmmo (Variables|Default|GetEquippedWeapon)) (Variables|Default|GetARAmmo))))))))))

(event Input|EnhancedActionEvents|EnhancedInputActionIA_Player_Fire
  (params (ActionValue :type Boolean) (ElapsedSeconds :type Float%20%28double-precision%29) (TriggeredSeconds :type Float%20%28double-precision%29) (InputAction :type Input%20Action%20Object%20Reference :default "/Game/01-Blueprints/Inputs/Actions/IA_Player_Fire.IA_Player_Fire"))
  (bind _equippedweapon (Variables|Default|GetEquippedWeapon))
  (bind _playeroverlayref (Variables|Default|GetPlayerOverlayRef))
  (bind _equippedweapon_2 (Variables|Default|GetEquippedWeapon))
  (bind _weaponmesh (Variables|/Game/01-Blueprints/Weapons/BP_Weapon.BP_Weapon_C|GetWeaponMesh _equippedweapon))
  ;[1 1 1] Fire input action - play animation - spawn bullet
  (:Started
    (if (Variables|Default|GetCanFire?)
      (Utilities|CheckCurrentAmmo?
        (:HaveAmmo
          (Variables|Default|SetCanFire? false)
          (Utilities|IsValid _equippedweapon
            (:Is%20Valid
              (Variables|Default|SetisFiring? true)
              (Components|Animation|PlayAnimation (Variables|Default|GetFirstPersonMesh) "/Game/FirstPersonArms/Animations/FP_Rifle_Fire.FP_Rifle_Fire" false)
              (Utilities|IsValid _weaponmesh
                (:Is%20Valid
                  (Components|Animation|PlayAnimation _weaponmesh "/Game/MilitaryWeapSilver/Weapons/Animations/Fire_Rifle_W.Fire_Rifle_W" false)
                  (Game|SpawnActorfromClass "/Game/01-Blueprints/Weapons/Bullets/BP_Bullets.BP_Bullets_C" (Math|Transform|MakeTransform (Transformation|GetSocketLocation (Variables|/Game/01-Blueprints/Weapons/BP_Weapon.BP_Weapon_C|GetWeaponMesh (Variables|Default|GetEquippedWeapon)) "BulletSpawn") (Transformation|GetSocketRotation (Variables|/Game/01-Blueprints/Weapons/BP_Weapon.BP_Weapon_C|GetWeaponMesh (Variables|Default|GetEquippedWeapon)) "BulletSpawn") "1.000000,1.000000,1.000000") "AdjustIfPossibleButAlwaysSpawn" "MultiplyWithRoot" 0 0)
                  (bind _result (Math|Integer|DecrementInt (Variables|/Game/01-Blueprints/Weapons/BP_Weapon.BP_Weapon_C|GetAmmo _equippedweapon_2))
                    (:%20%20
                      (Utilities|IsValid _playeroverlayref
                        (:Is%20Valid
                          (Default|UpdateAmmoText _playeroverlayref _result (Variables|Default|GetARAmmo))
                          (Utilities|FlowControl|Delay (Variables|/Game/01-Blueprints/Weapons/BP_Weapon.BP_Weapon_C|GetFireRate _equippedweapon_2))
                          (Variables|Default|SetCanFire? true)
                          (if (and (Variables|/Game/01-Blueprints/Weapons/BP_Weapon.BP_Weapon_C|GetisAutomatic? _equippedweapon_2) (Variables|Default|GetisFiring?))
                            (CallFunction|FireWeapon)))))))))))
        (:NoAmmoLeft
          (CallFunction|Reload)
          (Variables|Default|SetisFiring? false)))))
  (:Completed
    (Variables|Default|SetisFiring? false)))

(event Input|EnhancedActionEvents|EnhancedInputActionIA_Player_Reload
  (params (ActionValue :type Boolean) (ElapsedSeconds :type Float%20%28double-precision%29) (TriggeredSeconds :type Float%20%28double-precision%29) (InputAction :type Input%20Action%20Object%20Reference :default "/Game/01-Blueprints/Inputs/Actions/IA_Player_Reload.IA_Player_Reload"))
  (bind _equippedweapon (Variables|Default|GetEquippedWeapon))
  (bind _playeroverlayref (Variables|Default|GetPlayerOverlayRef))
  (bind _equippedweapon_2 (Variables|Default|GetEquippedWeapon))
  ;[1 1 1] Reload
  (:Started
    (if (not (Variables|Default|GetisReloading?))
      (Variables|Default|SetisReloading? true)
      (Variables|Default|SetCanFire? false)
      (Utilities|IsValid _equippedweapon_2
        (:Is%20Valid
          (bind _output_get (Variables|Default|SetARAmmo (+ (Variables|Default|GetARAmmo) (Variables|/Game/01-Blueprints/Weapons/BP_Weapon.BP_Weapon_C|GetAmmo _equippedweapon_2))))
          (if (> _output_get 0)
            (if (< (- (Variables|Default|GetARAmmo) (Variables|/Game/01-Blueprints/Weapons/BP_Weapon.BP_Weapon_C|GetMaxAmmo _equippedweapon_2)) 0)
              (Variables|Default|SetARAmmo (* (Variables|Default|GetARAmmo) -1)))
            (bind _output_get_2 (Variables|/Game/01-Blueprints/Weapons/BP_Weapon.BP_Weapon_C|SetAmmo (Variables|Default|GetEquippedWeapon) (Math|Integer|Clamp(Integer) (Variables|Default|GetARAmmo) 0 (Variables|/Game/01-Blueprints/Weapons/BP_Weapon.BP_Weapon_C|GetMaxAmmo (Variables|Default|GetEquippedWeapon)))))
            (if (> (- _output_get_2 (Variables|Default|GetARAmmo)) 0)
              (Variables|/Game/01-Blueprints/Weapons/BP_Weapon.BP_Weapon_C|SetAmmo (Variables|Default|GetEquippedWeapon) (- _output_get_2 (Variables|Default|GetARAmmo)))
              (Variables|Default|SetARAmmo 0)
              (else
                (Variables|Default|SetARAmmo (* (- _output_get_2 (Variables|Default|GetARAmmo)) -1))))
            (Utilities|IsValid _playeroverlayref
              (:Is%20Valid
                (Default|UpdateAmmoText _playeroverlayref (Variables|/Game/01-Blueprints/Weapons/BP_Weapon.BP_Weapon_C|GetAmmo _equippedweapon) (Variables|Default|GetARAmmo))
                (Utilities|FlowControl|Delay (Variables|/Game/01-Blueprints/Weapons/BP_Weapon.BP_Weapon_C|GetReloadCD _equippedweapon))
                (Variables|Default|SetCanFire? true)
                (Variables|Default|SetisReloading? false)))))))))

(event EventBeginPlay
  ;[1 1 1] Begin Play - Add mapping context to IMC PLAYER
  (bind _asplayer_controller (Utilities|Casting|CastToPlayerController (Game|GetPlayerController 0)))
  (Utilities|IsValid (PlayerController|LocalPlayerSubsystems|GetEnhancedInputLocalPlayerSubsystem _asplayer_controller)
    (:Is%20Valid
      (Input|AddMappingContext (PlayerController|LocalPlayerSubsystems|GetEnhancedInputLocalPlayerSubsystem _asplayer_controller) "/Game/01-Blueprints/Inputs/IMC_Player.IMC_Player" 0 "(bIgnoreAllPressedKeysUntilRelease=True,bForceImmediately=False,bNotifyUserSettings=False)")
      (bind _returnvalue (UserInterface|CreateWidget "/Game/01-Blueprints/Widgets/WBP_PlayerOverlay.WBP_PlayerOverlay_C"))
      (bind _output_get (Variables|Default|SetPlayerOverlayRef _returnvalue))
      (UserInterface|Viewport|AddtoViewport _output_get 0)
      (Default|UpdateHealth (Variables|Default|GetPlayerOverlayRef) (Variables|Default|GetCurrentHealth) (Variables|Default|GetMaxHealth)))))

(event Input|KeyboardEvents|U
  (params (Key :type Key%20Structure :default "None"))
  (:Pressed
    (CallFunction|PlayerDamage 15.0)))

(fn ConstructionScript)